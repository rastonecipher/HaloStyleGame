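; Aim assist component that nudges the first-person player's control rotation when aiming at objects of a specific object type.
; When started enabled, a narrow capsule trace along the camera's forward vector gates a much wider one, whose hit drives the correction.
; The controller rotation slowly interpolates toward the direction from that impact point to slightly above the hit actor's origin, rather than from the camera to the target.
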(event `Start`
  (params (Enabled :type Boolean))
  (if Enabled
    (bind _returnvalue (`self.AimAssistTrace` 8.0))
    (if _returnvalue
      (bind (_returnvalue_2 _outhit) (`self.AimAssistTrace` 128.0))
      (if _returnvalue_2
        (`self.AimAssistRotation` _outhit)))))

(fn `AimAssistRotation`
  (params (Hit :type "HitResult Structure"))
  (bind _returnvalue (`GameplayStatics.GetPlayerController` 0))
  (bind (_bblockinghit _binitialoverlap _time _location _impactpoint _normal _impactnormal _physmat _hitactor) (`GameplayStatics.BreakHitResult` Hit))
  (`Controller.SetControlRotation` _returnvalue (`KismetMathLibrary.RInterpTo` (`Controller.GetControlRotation` _returnvalue) (`KismetMathLibrary.Conv_VectorToRotator` (`KismetMathLibrary.Normal` (- (+ (`Actor.K2_GetActorLocation` _hitactor) (0.0 0.0 50.0)) _impactpoint))) (`GameplayStatics.GetWorldDeltaSeconds`) 0.5)))

(fn `AimAssistTrace`
  (params (Radius :type "Float (double-precision)"))
  (returns (ReturnValue :type Boolean) (OutHit :type "HitResult Structure"))
  (bind _firstpersoncamera (`/Game/FPS_Game/Blueprints/BP_CharacterBase.FirstPersonCamera` (`/Game/FPS_Game/Blueprints/System/BP_Library.GetPlayerCast`)))
  (bind _returnvalue (`SceneComponent.K2_GetComponentLocation` _firstpersoncamera))
  (bind (_outhit _returnvalue_2) (`KismetSystemLibrary.CapsuleTraceSingleForObjects` _returnvalue (+ _returnvalue (* (`SceneComponent.GetForwardVector` _firstpersoncamera) 1500.0)) Radius Radius (`|MakeArray` "ObjectTypeQuery7" :!type "EObjectTypeQuery Enum")))
  (return _returnvalue_2 _outhit))